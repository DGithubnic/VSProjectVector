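; BP_PortalManager is a manager Blueprint that drives the view through a portal between two screen actors, Screen1 and Screen2.
; Each tick, Screen1Update moves and rotates Screen2's PortalCapture to match the player camera's pose relative to Screen1, re-expressed at Screen2.
; The transfer uses the rotation delta between both screen roots, with Screen2's yaw turned 180 degrees.
; Only this one direction is updated.
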(event `self.ReceiveTick`
  (params (DeltaSeconds :type "Float (single-precision)"))
  (`self.Screen 1 Update`))

(fn `Screen 1 Update`
  (bind _defaultsceneroot (`/Game/VSPProject/VSP_BluePrint/BP_Screen2.DefaultSceneRoot` (`self.Screen2`)))
  (bind _defaultsceneroot_2 (`/Game/VSPProject/VSP_BluePrint/BP_Screen1.DefaultSceneRoot` (`self.Screen1`)))
  (bind _transformcomponent (`PlayerCameraManager.TransformComponent` (`GameplayStatics.GetPlayerCameraManager` 0)))
  (bind (_returnvalue_roll _returnvalue_pitch _returnvalue_yaw) (`KismetMathLibrary.BreakRotator` (`SceneComponent.K2_GetComponentRotation` _defaultsceneroot)))
  (bind _returnvalue (`KismetMathLibrary.NormalizedDeltaRotator` (`KismetMathLibrary.MakeRotator` _returnvalue_roll _returnvalue_pitch (- _returnvalue_yaw 180.0)) (`SceneComponent.K2_GetComponentRotation` _defaultsceneroot_2)))
  (`SceneComponent.K2_SetWorldLocationAndRotation` (`/Game/VSPProject/VSP_BluePrint/BP_Screen2.PortalCapture` (`self.Screen2`)) (+ (- (`SceneComponent.K2_GetComponentLocation` _defaultsceneroot) (`KismetMathLibrary.GreaterGreater_VectorRotator` (`SceneComponent.K2_GetComponentLocation` _defaultsceneroot_2) _returnvalue)) (`KismetMathLibrary.GreaterGreater_VectorRotator` (`SceneComponent.K2_GetComponentLocation` _transformcomponent) _returnvalue)) (`KismetMathLibrary.ComposeRotators` (`SceneComponent.K2_GetComponentRotation` _transformcomponent) _returnvalue) false false))

(fn `UserConstructionScript`)