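; BP_MonsterSpawner is a spawner actor that places batches of BP_Monster1 in the level, away from the player.
; SpawnMonster picks random world positions in a fixed rectangle at constant height, re-rolling any that fall too close to the player character.
; A looping timer to call SpawnMonster exists but is disconnected from the empty BeginPlay, so this Blueprint does not trigger spawning itself.
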(event `self.ReceiveBeginPlay`
  ;[1 1 1] SpawnMonster 함수를 호출
)

(fn `SpawnMonster`
  ;[1 1 1] 몬스터 스폰(1800범위 내에는 소환x)
  (for _ (range 5)
    (bind _output_get (set `self.MonsterPosition` (`KismetMathLibrary.MakeVector` (`KismetMathLibrary.RandomFloatInRange` -5000.0 5000.0) (`KismetMathLibrary.RandomFloatInRange` -1500.0 1500.0) 60.0) :!label _label))
    (if (< 1800.0 (`KismetMathLibrary.Vector_Distance` _output_get (`self.K2_GetActorLocation` (`GameplayStatics.GetPlayerCharacter` 0))))
      (`|SpawnActorFromClass` "/Game/VSPProject/VSP_BluePrint/BP_Monster1.BP_Monster1_C" (`KismetMathLibrary.MakeTransform` (`self.MonsterPosition`)) "Undefined" "OverrideRootScale" null null)
      (else
        (goto _label)))))

(fn `UserConstructionScript`)